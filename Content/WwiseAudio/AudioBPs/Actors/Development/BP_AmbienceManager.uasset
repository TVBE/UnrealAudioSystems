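; Ambience manager for BP_WorldAudio that spawns procedural one-shot bird, insect and misc sounds around the player, initialized only off dedicated servers.
; On BiomeUpdate it clears timers, loads the biome's DataTable row and starts a randomized, self-rescheduling timer per validated sound type.
; Each timer plays a random day or night event at a random offset from the pawn, outside an exclusion radius.
; The Misc type has no row data wired.
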(event `Event SpawnBirds_Far`
  ;[1 1 1] Event SpawnBirds_Far
  (`self.PlaySoundSource` "NewEnumerator1")
  (`self.SetSpawnTimer` "NewEnumerator1" (delegate `Event SpawnBirds_Far`)))

(event `self.ReceiveBeginPlay`
  ;[1 1 1] Event BeginPlay
  (if (not (`KismetSystemLibrary.IsDedicatedServer`))
    (`self.Initialize`)))

(event `Event BiomeUpdate`
  (params (Biome :type "/Game/WwiseAudio/AudioBPs/Actors/Development/BPE_AudioBiome Enum" :default "NewEnumerator0"))
  ;[1 1 1] Event BiomeUpdate
  (`self.ClearTimers`)
  (`self.UpdateBiomeData` Biome)
  (`self.InitializeTimers`))

(event `Event SpawnBirds_Close`
  ;[1 1 1] Event SpawnBirds_Close
  (`self.PlaySoundSource` "NewEnumerator2")
  (`self.SetSpawnTimer` "NewEnumerator2" (delegate `Event SpawnBirds_Close`)))

(event `Event SpawnInsects`
  ;[1 1 1] Event SpawnInsects
  (`self.PlaySoundSource` "NewEnumerator0")
  (`self.SetSpawnTimer` "NewEnumerator0" (delegate `Event SpawnInsects`)))

(event `Event SpawnMisc`
  ;[1 1 1] Event SpawnMisc
  (`self.PlaySoundSource` "NewEnumerator3")
  (`self.SetSpawnTimer` "NewEnumerator3" (delegate `Event SpawnMisc`)))

(fn `ClearTimers`
  (for _array_element (`self.TimerHandles`)
    (if (`KismetSystemLibrary.K2_IsTimerActiveHandle` _array_element)
      (`KismetSystemLibrary.K2_ClearAndInvalidateTimerHandle` _array_element))))

(fn `GetRelevantSoundSourceData`
  (params (Type :type "/Game/WwiseAudio/AudioBPs/Actors/Development/BPE_ProceduralAudioType Enum" :default "NewEnumerator1") (TimeOfDay :type "/Game/WwiseAudio/AudioBPs/Actors/Development/BPE_TimeOfDay Enum" :default "NewEnumerator0"))
  (returns (ReturnValue :type "/Game/WwiseAudio/AudioBPs/Actors/Development/BPS_SoundSourceData Structure"))
  (bind (_birds_far _birds_close _insects) (break `/Game/WwiseAudio/AudioBPs/Actors/Development/BPS_BiomeAudioData` (`self.CurrentDataRow`)))
  (bind (_day _night) (break `/Game/WwiseAudio/AudioBPs/Actors/Development/BPS_ProceduralAudioData` (select `/Game/WwiseAudio/AudioBPs/Actors/Development/BPE_ProceduralAudioType` Type :`NewEnumerator1` _birds_far :`NewEnumerator2` _birds_close :`NewEnumerator0` _insects)))
  (return (select `/Game/WwiseAudio/AudioBPs/Actors/Development/BPE_TimeOfDay` (`local.TimeOfDay`) :`NewEnumerator0` _day :`NewEnumerator1` _night)))

(fn `GetSoundSourceTransform`
  (params (Type :type "/Game/WwiseAudio/AudioBPs/Actors/Development/BPE_ProceduralAudioType Enum" :default "NewEnumerator1"))
  (returns (NewParam :type "Transform Structure"))
  (bind _returnvalue (`Controller.K2_GetPawn` (`GameplayStatics.GetPlayerController` 0)))
  (`/Engine/EditorBlueprintResources/StandardMacros.IsValid` _returnvalue
    (:`Is Valid`
      (return (`KismetMathLibrary.Conv_VectorToTransform` (select `/Game/WwiseAudio/AudioBPs/Actors/Development/BPE_ProceduralAudioType` Type :`NewEnumerator1` (`self.RandomVectorAroundActor` _returnvalue (0.0 0.0 400.0) false 3000.0 3000.0 150.0 2000.0) :`NewEnumerator2` (`self.RandomVectorAroundActor` _returnvalue (0.0 0.0 0.0) false 1500.0 1500.0 250.0 800.0) :`NewEnumerator0` (`self.RandomVectorAroundActor` _returnvalue (0.0 0.0 -50.0) false 900.0 900.0 50.0 500.0) :`NewEnumerator3` (`self.RandomVectorAroundActor` _returnvalue (0.0 0.0 0.0) false 1000.0 1000.0 100.0 500.0)))))))

(fn `GetSpawnInterval`
  (params (Density :type "Float (double-precision)") (`Storm Multiplier` :type "Float (double-precision)") (Type :type "/Game/WwiseAudio/AudioBPs/Actors/Development/BPE_ProceduralAudioType Enum" :default "NewEnumerator1"))
  (returns (ReturnValue :type "Float (double-precision)"))
  (bind _returnvalue (* (* (- 1.0 Density) 4.0) `Storm Multiplier`))
  (return (`KismetMathLibrary.RandomFloatInRange` (* _returnvalue 0.9) (* _returnvalue 1.1))))

(fn `Initialize`
  (bind _returnvalue (`Actor.GetComponentByClass` (`self.Owner`) "/Game/WwiseAudio/AudioBPs/Actors/Development/BP_SoundSourceManager.BP_SoundSourceManager_C"))
  (`|ExecutionSequence`
    (:`then_0`
      ;[1 1 1] Get owner as BP_WorldAudio.
      (bind _asbp_world_audio (cast `/Game/WwiseAudio/AudioBPs/Actors/Development/BP_WorldAudio` (`self.GetOwner`)))
      (set `self.Owner` _asbp_world_audio))
    (:`then_1`
      ;[1 1 1] Get reference to SoundSourcePool from owner.
      (`/Engine/EditorBlueprintResources/StandardMacros.IsValid` _returnvalue
        (:`Is Valid`
          (set `self.SoundSourcePool` _returnvalue))))
    (:`then_4`
      ;[1 1 1] Finalize.
      (set `self.IsInitialized` true))))

(fn `InitializeTimers`
  (`|ExecutionSequence`
    (:`then_0`
      ;[1 1 1] Set timer for Birds_Far.
      (`self.SetSpawnTimer` "NewEnumerator1" (`|CreateDelegate` :!event `Event SpawnBirds_Far`)))
    (:`then_1`
      ;[1 1 1] Set timer for Birds_Close.
      (`self.SetSpawnTimer` "NewEnumerator2" (`|CreateDelegate` :!event `Event SpawnBirds_Close`)))
    (:`then_2`
      ;[1 1 1] Set timer for Birds_Close.
      (`self.SetSpawnTimer` "NewEnumerator0" (`|CreateDelegate` :!event `Event SpawnInsects`)))
    (:`then_3`
      ;[1 1 1] Set timer for Birds_Close.
      (`self.SetSpawnTimer` "NewEnumerator3" (`|CreateDelegate` :!event `Event SpawnMisc`)))))

(fn `PlaySoundSource`
  (params (Type :type "/Game/WwiseAudio/AudioBPs/Actors/Development/BPE_ProceduralAudioType Enum" :default "NewEnumerator1"))
  (locals (Transform :type "Transform Structure"))
  (bind _returnvalue (`self.GetRelevantSoundSourceData` Type (`self.TimeOfDay`)))
  (bind (_use _delaymin _delaymax _maxinstances _storm_multiplier _events) (break `/Game/WwiseAudio/AudioBPs/Actors/Development/BPS_SoundSourceData` _returnvalue))
  (if _use
    (bind _output_get (set `local.Transform` (`self.GetSoundSourceTransform` Type)))
    (`self.PlaySoundSourceAtLocation` (`KismetArrayLibrary.Array_Random` _events) _output_get)
    (if (== (`KismetMathLibrary.Conv_ByteToInt` (`self.Debug Level`)) 3)
      (`KismetSystemLibrary.DrawDebugCircle` (.location (`local.Transform`)) 100.0 12 (struct :`B` 1.0 :`A` 1.0) 4.0 1.0))))

(fn `PrintDebugString`
  (params (String :type String) (DebugLevel :type "/Game/WwiseAudio/AudioBPs/Actors/Development/BPE_ActorDebugLevel Enum" :default "NewEnumerator2") (Duration :type "Float (double-precision)" :default 6.0))
  (if (<= (`KismetMathLibrary.Conv_ByteToInt` DebugLevel) (`KismetMathLibrary.Conv_ByteToInt` (`self.Debug Level`)))
    (`KismetSystemLibrary.PrintString` (`local.String`) true true (struct :`B` 1.0 :`A` 1.0) (`local.Duration`))))

(fn `RandomVectorAroundActor`
  (params (Target :type "Actor Object Reference") (Offset :type "Vector Structure") (UseActorOrientation :type Boolean) (XRange :type "Float (double-precision)") (YRange :type "Float (double-precision)") (ZRange :type "Float (double-precision)") (ExclusionRadius :type "Float (double-precision)") (__WorldContext :type "Object Object Reference"))
  (returns (ReturnValue :type "Vector Structure"))
  (bind _returnvalue (`KismetMathLibrary.RandomFloatInRange` ExclusionRadius YRange))
  (bind _returnvalue_2 (`KismetMathLibrary.RandomFloatInRange` ExclusionRadius XRange))
  (bind _returnvalue_3 (`Actor.K2_GetActorLocation` Target))
  (bind _returnvalue_4 (`KismetMathLibrary.SelectFloat` (- 0.0 _returnvalue) _returnvalue (`KismetMathLibrary.RandomBool`)))
  (bind _returnvalue_5 (`KismetMathLibrary.SelectFloat` (- 0.0 _returnvalue_2) _returnvalue_2 (`KismetMathLibrary.RandomBool`)))
  (return (+ (`KismetMathLibrary.SelectVector` (+ _returnvalue_3 (+ (* (`Actor.GetActorRightVector` Target) _returnvalue_4) (* (`Actor.GetActorForwardVector` Target) _returnvalue_5))) (`KismetMathLibrary.MakeVector` (+ (.x _returnvalue_3) _returnvalue_5) (+ (.y _returnvalue_3) _returnvalue_4) (+ (.z _returnvalue_3) (`KismetMathLibrary.RandomFloatInRange` (* ZRange -1.0) ZRange))) UseActorOrientation) Offset)))

(fn `SetSpawnTimer`
  (params (Type :type "/Game/WwiseAudio/AudioBPs/Actors/Development/BPE_ProceduralAudioType Enum" :default "NewEnumerator1") (Event :type Delegate))
  (bind _returnvalue (`self.GetRelevantSoundSourceData` Type (`self.TimeOfDay`)))
  (bind (_use _delaymin _delaymax) (break `/Game/WwiseAudio/AudioBPs/Actors/Development/BPS_SoundSourceData` _returnvalue))
  (if _use
    (if (`self.ValidateSoundSourceData` _returnvalue Type (`self.TimeOfDay`))
      (bind _returnvalue_2 (`KismetSystemLibrary.K2_SetTimerDelegate` Event (`KismetMathLibrary.RandomFloatInRange` _delaymin _delaymax)))
      (`KismetArrayLibrary.Array_Add` (`self.TimerHandles`) _returnvalue_2))))

(fn `UpdateBiomeData`
  (params (Biome :type "/Game/WwiseAudio/AudioBPs/Actors/Development/BPE_AudioBiome Enum" :default "NewEnumerator0"))
  (bind _output_get (set `self.Biome` Biome))
  ;[1 1 1] Get DataTable row.
  (bind _returnvalue (`|GetDataTableRow` (`self.DataTable`) (`KismetStringLibrary.Conv_StringToName` (`|GetEnumeratorNameAsString` _output_get)))
    (:`then`
      (set `self.CurrentDataRow` _returnvalue)
      (if (>= (`KismetMathLibrary.Conv_ByteToInt` (`self.Debug Level`)) 2)
        (`KismetSystemLibrary.PrintString` (`KismetTextLibrary.Conv_TextToString` (`|FormatText` (`KismetSystemLibrary.GetDisplayName` self) "{self}: Audio biome changed to:{biome}" (`|GetEnumeratorName` (`self.Biome`)))) true true (struct :`B` 1.0 :`A` 1.0) 5.0)))))

(fn `UpdateSpawners`
  (`|ExecutionSequence`
    (:`then_0`
      (`self.GetRelevantSoundSourceData` "NewEnumerator2"))))

(fn `ValidateSoundSourceData`
  (params (Input :type "/Game/WwiseAudio/AudioBPs/Actors/Development/BPS_SoundSourceData Structure") (Type :type "/Game/WwiseAudio/AudioBPs/Actors/Development/BPE_ProceduralAudioType Enum" :default "NewEnumerator1") (TimeOfDay :type "/Game/WwiseAudio/AudioBPs/Actors/Development/BPE_TimeOfDay Enum" :default "NewEnumerator0"))
  (returns (ReturnValue :type Boolean))
  (bind (_use _delaymin _delaymax _maxinstances _storm_multiplier _events) (break `/Game/WwiseAudio/AudioBPs/Actors/Development/BPS_SoundSourceData` Input))
  ;[1 1 1] Check whether this BPS_SoundSourcedata contains valid attributes to be used for the spawner.
  (if (== _use true)
    (if (and (> _delaymin 0.0) (> _delaymax 0.0) (< _delaymin _delaymax) (> _maxinstances 0) (>= _storm_multiplier 0.0) (`KismetArrayLibrary.Array_IsNotEmpty` _events))
      (return true))
    (else
      (`self.PrintDebugString` (`KismetTextLibrary.Conv_TextToString` (`|FormatText` "{Self}: Warning! The procedural SoundSource data for row {DataRow} for type {Type} at {TimeOfDay} contains invalid atributes. {Type} will not play for this audio biome untill fixed." (`KismetSystemLibrary.GetDisplayName` self) (`|GetEnumeratorNameAsString` (`self.Biome`)) (`|GetEnumeratorNameAsString` (`local.Type`)) (`|GetEnumeratorNameAsString` (`local.TimeOfDay`)))))
      (return false))))