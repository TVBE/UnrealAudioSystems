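; BP_WorldAudio is an in-development world audio actor meant to poll the player's location as they move.
; On BeginPlay, outside dedicated servers, it destroys itself if another instance exists and sets an initialized flag.
; DecidePoll uses a squared-distance threshold from the last poll position to trigger PollLocation and a debug print.
; PollLocation is an empty stub, and nothing in this graph calls DecidePoll.
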(event `self.ReceiveBeginPlay`
  ;[1 1 1] Event Begin Play
  (if (not (`KismetSystemLibrary.IsDedicatedServer`))
    (`self.Initialize`)))

(fn `DecidePoll`
  (locals (Location :type "Vector Structure" :default (0.0 0.0 0.0)))
  (bind _returnvalue (`GameplayStatics.GetPlayerPawn` 0))
  (`/Engine/EditorBlueprintResources/StandardMacros.IsValid` _returnvalue
    (:`Is Valid`
      (bind _output_get (set `local.Location` (`self.K2_GetActorLocation` _returnvalue)))
      (if (> (`KismetMathLibrary.Vector_DistanceSquared` _output_get (`self.LastPollLocation`)) 100000000.0)
        (`self.PollLocation`)
        (set `self.LastPollLocation` (`local.Location`))
        (`KismetSystemLibrary.PrintString` "Doing New Poll!")))))

(fn `Initialize`
  (`|ExecutionSequence`
    (:`then_0`
      ;[1 1 1] Make sure that there is currently only one instance of this Blueprint in the world.
      (bind _outactors (`GameplayStatics.GetAllActorsOfClass` (`GameplayStatics.GetObjectClass` self)))
      (if (> (`KismetArrayLibrary.Array_Length` _outactors) 1)
        (`self.K2_DestroyActor` self)))
    (:`then_1`
      (set `self.isInitialized` true))))

(fn `PollLocation`)

(fn `UserConstructionScript`)