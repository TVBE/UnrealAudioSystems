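; Development spline-based audio ambience zone actor that carries a Biome component, with runtime audio logic still stubbed out.
; Construction adds the Biome class component and builds editor-visible, game-hidden, colored spline meshes to show the boundary.
; A dot product against the spline's right vector tests whether the player is inside, but the overlap update takes no action on it.
; Helpers provide player-to-spline distance and emitter debug drawing, and BeginPlay prints the biome component's name after a delay.
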(event `self.ReceiveBeginPlay`
  ;[1 1 1] Event Beginplay
  (`KismetSystemLibrary.Delay` 8.0)
  (`KismetSystemLibrary.PrintString` (`KismetSystemLibrary.GetDisplayName` (`self.BP_Audio_BiomeComponent`)) true true (struct :`R` 0.01193 :`G` 1.0 :`A` 1.0) 10.0))

(event `self.UpdateActorState`
  (params (`isOverlapping?` :type Boolean))
  (if `isOverlapping?`
    (if (`self.GetIsInsideSpline`)
      _)))

(fn `AddBiomeComponent`)

(fn `DrawDebugVisualisation`
  (bind _ak_emitter_location (`self.Ak Emitter Location`))
  (`KismetSystemLibrary.DrawDebugConeInDegrees` _ak_emitter_location (`KismetMathLibrary.Conv_RotatorToVector` (`PlayerCameraManager.GetCameraRotation` (`PlayerController.PlayerCameraManager` (`GameplayStatics.GetPlayerController` 0)))) 100.0 45.0 45.0 12 (struct :`R` 1.0 :`G` 1.0 :`B` 1.0 :`A` 1.0) 0.0 2.0)
  (`KismetSystemLibrary.DrawDebugSphere` _ak_emitter_location 10.0 12 (struct :`G` 0.344682 :`B` 1.0 :`A` 1.0) 0.0 4.0))

(fn `GetDistanceToPlayerFromClosestSplinePoint`
  (returns (DistanceToPlayerFromClosestSplinePoint :type "Float (double-precision)"))
  (bind _returnvalue (`self.K2_GetActorLocation` (`GameplayStatics.GetPlayerPawn` 0)))
  (return (`KismetMathLibrary.VSize` (- (`SplineComponent.FindLocationClosestToWorldLocation` (`self.Spline`) _returnvalue "World") _returnvalue))))

(fn `GetIsInsideSpline`
  (returns (`IsInsideSpline?` :type Boolean))
  (locals (PlayerPawnLocation :type "Vector Structure"))
  (bind _returnvalue (`GameplayStatics.GetPlayerPawn` 0))
  (`/Engine/EditorBlueprintResources/StandardMacros.IsValid` _returnvalue
    (:`Is Valid`
      (set `local.PlayerPawnLocation` (`self.K2_GetActorLocation` _returnvalue))
      (return (> (`KismetMathLibrary.Dot_VectorVector` (- (`self.Spline Curve Location Closest To Player`) (`local.PlayerPawnLocation`)) (`SplineComponent.FindRightVectorClosestToWorldLocation` (`self.Spline`) (`local.PlayerPawnLocation`) "World")) 0.0)))))

(fn `SetComponents`
  (bind _biome (`self.Biome`))
  (`|ExecutionSequence`
    (:`then_0`
      (set `self.useBiome?` (`KismetSystemLibrary.IsValidClass` _biome))
      (bind _returnvalue (`|AddComponentByClass` _biome))
      (set `self.BP_Audio_BiomeComponent` _returnvalue))))

(fn `SetSplineMesh`
  (locals (SplineMeshComponent :type "SplineMeshComponent Object Reference"))
  (bind _returnvalue (`KismetMathLibrary.MakeVector2D` 1.0 3.0))
  (bind _spline (`self.Spline`))
  (for _index (range (`SplineComponent.GetNumberOfSplinePoints` (`self.Spline`)))
    (bind _returnvalue_2 (`AddComponent|NODE_AddSplineMeshComponent-1`)) ; Click node for details. We use a transparent material
    (set `local.SplineMeshComponent` _returnvalue_2)
    (bind _returnvalue_3 (`PrimitiveComponent.CreateDynamicMaterialInstance` (`local.SplineMeshComponent`) 0 "/Game/WwiseAudio/AudioBPs/Resources/M_DebugMaterial01.M_DebugMaterial01" "None"))
    (`MaterialInstanceDynamic.SetVectorParameterValue` _returnvalue_3 "Base Color Parameter" (`self.Color`)) ; Set the color of the mesh
    (`SplineMeshComponent.SetStartScale` (`local.SplineMeshComponent`) _returnvalue true)
    (`SplineMeshComponent.SetEndScale` (`local.SplineMeshComponent`) _returnvalue true)
    (bind (_location _tangent) (`SplineComponent.GetLocationAndTangentAtSplinePoint` _spline _index "Local"))
    (bind (_location_2 _tangent_2) (`SplineComponent.GetLocationAndTangentAtSplinePoint` _spline (+ _index 1) "Local"))
    (`SplineMeshComponent.SetStartAndEnd` (`local.SplineMeshComponent`) _location _tangent _location_2 _tangent_2 true)
    (`SceneComponent.SetHiddenInGame` (`local.SplineMeshComponent`) true false)))

(fn `UserConstructionScript`
  (`|ExecutionSequence`
    (:`then_0`
      (if (`self.isVisibleInEditor?`)
        (`self.SetSplineMesh`) ; Editor visualisation
      ))
    (:`then_1`
      (`self.SetComponents`))))