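; BP_SoundSourceManager is a component on BP_WorldAudio that plays audio events at world locations through a pool of BP_SoundSource actors.
; On non-server instances, it binds to the PostEventAtLocation dispatcher of the owner's BP_AmbienceManager.
; Play requests move and reuse a pooled source, or spawn and initialize a new one with a debug print when the pool is empty.
; Sources return to the pool through a release event.
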(event `self.ReceiveBeginPlay`
  ;[1 1 1] Event Begin Play
  (if (not (`KismetSystemLibrary.IsDedicatedServer`))
    (`self.Initialize`)))

(event `/Game/WwiseAudio/AudioBPs/Interfaces/BPI_SoundSource.ReleaseBackToPool`
  (params (Input :type "/Game/WwiseAudio/AudioBPs/Actors/Development/BP_SoundSource Object Reference"))
  ;[1 1 1] Event Release Back to Pool
  (`KismetArrayLibrary.Array_Add` (`self.Pool`) Input))

(event `PlaySoundAtLocation`
  (params (Event :type "AkAudioEvent Object Reference") (Transform :type "Transform Structure"))
  (bind _output (`|GetArrayItem` (`self.Pool`)))
  ;[1 1 1] Event Play Sound At Location
  (if (`KismetArrayLibrary.Array_IsValidIndex` (`self.Pool`))
    (`Actor.K2_SetActorTransform` _output Transform false false)
    (`/Game/WwiseAudio/AudioBPs/Actors/Development/BP_SoundSource.PostEvent` _output Event)
    (`KismetArrayLibrary.Array_Remove` (`self.Pool`))
    (else
      (bind _returnvalue (`|SpawnActorFromClass` "/Game/WwiseAudio/AudioBPs/Actors/Development/BP_SoundSource.BP_SoundSource_C" Transform "Undefined" "OverrideRootScale" null null))
      (`/Game/WwiseAudio/AudioBPs/Actors/Development/BP_SoundSource.Initialize` _returnvalue self)
      (`/Game/WwiseAudio/AudioBPs/Actors/Development/BP_SoundSource.PostEvent` _returnvalue Event)
      (`KismetSystemLibrary.PrintString` "Created new SoundSource!!!!"))))

(fn `Initialize`
  (bind _returnvalue (`Actor.GetComponentByClass` (`self.Owner`) "/Game/WwiseAudio/AudioBPs/Actors/Development/BP_AmbienceManager.BP_AmbienceManager_C"))
  (`|ExecutionSequence`
    (:`then_0`
      ;[1 1 1] Get owner as BP_WorldAudio
      (bind _asbp_world_audio (cast `/Game/WwiseAudio/AudioBPs/Actors/Development/BP_WorldAudio` (`self.GetOwner`)))
      (set `self.Owner` _asbp_world_audio))
    (:`then_1`
      ;[1 1 1] Get BP_SoundSourceManager from owner.
      (`/Engine/EditorBlueprintResources/StandardMacros.IsValid` _returnvalue
        (:`Is Valid`
          (set `self.SoundsourceManager` _returnvalue))))
    (:`then_2`
      ;[1 1 1] Subscribe to events.
      (add `/Game/WwiseAudio/AudioBPs/Actors/Development/BP_AmbienceManager.PostEventAtLocation` (`self.SoundsourceManager`) (`|CreateDelegate` :!event `PlaySoundAtLocation`)))))