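; BP_SoundSource is a development, poolable Wwise sound emitter that posts events on its AkComponent.
; PostEvent skips invalid events and dedicated servers, flags itself as playing and registers an end-of-event callback.
; The callback clears the flag and releases the actor to the pool supplied through Initialize.
; BeginPlay also posts a hardcoded crocodile death event after a short delay, apparently as a test.
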(event `self.ReceiveBeginPlay`
  (`KismetSystemLibrary.Delay` 6.0)
  (`self.PostEvent` "/Game/WwiseAudio/Events/Animals/Animals_Crocodile/Animal_Crocodile_Death.Animal_Crocodile_Death"))

(event `PostEvent`
  (params (Event :type "AkAudioEvent Object Reference"))
  ;[1 1 1] Event Post Event
  (if (and (`KismetSystemLibrary.IsValid` Event) (not (`KismetSystemLibrary.IsDedicatedServer`)))
    (`AkGameObject.PostAkEvent` :`self` (`self.AkComponent`) :`AkEvent` Event :`CallbackMask` 1 :`PostEventCallback` (`|CreateDelegate` :!event `Event Callback`))
    (set `self.IsPlaying` true)))

(event `Event Callback`
  (params (CallbackType :type "EAkCallbackType Enum" :default "EndOfEvent") (CallbackInfo :type "AkCallbackInfo Object Reference"))
  ;[1 1 1] Event Callback
  (set `self.IsPlaying` false)
  (`/Engine/EditorBlueprintResources/StandardMacros.IsValid` (`self.Pool`)
    (:`Is Valid`
      (`self.ReleaseBackToPool` (`self.Pool`) self))))

(fn `Initialize`
  (params (Pool :type "/Game/WwiseAudio/AudioBPs/Actors/Development/BP_SoundSourceManager Object Reference"))
  (set `self.Pool` Pool))

(fn `UserConstructionScript`)