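; Actor component for collision audio on a StaticMeshActor, still unfinished: it detects hits, but SetMetaSoundAttributes is empty and hits never drive the sound.
; On BeginPlay it binds OnActorHit and adds an AudioComponent with a MetaSound source.
; Hits whose mass-normalized impulse exceeds a threshold start a cooldown and enable component Tick.
; Tick clears the cooldown, then disables itself after a few idle seconds.
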(event `self.ReceiveBeginPlay`
  ;[1 1 1] Evet BeginPlay
  (`self.Initialize`))

(event `self.ReceiveTick`
  (params (DeltaSeconds :type "Float (single-precision)"))
  ;[1 1 1] Event Tick
  (`self.Update` DeltaSeconds))

(fn `GetHitForceScale`
  (params (SelfActor :type "Actor Object Reference") (OtherActor :type "Actor Object Reference") (NormalImpulse :type "Vector Structure"))
  (returns (ReturnValue :type Integer64))
  (return (`KismetMathLibrary.Conv_DoubleToInt64` (`KismetMathLibrary.VSize` (/ (`local.NormalImpulse`) (`PrimitiveComponent.GetMass` (`StaticMeshActor.StaticMeshComponent` (`self.StaticMesh`))))))))

(fn `HandleCollision`
  (params (SelfActor :type "Actor Object Reference") (OtherActor :type "Actor Object Reference") (NormalImpulse :type "Vector Structure") (Hit :type "HitResult Structure (by ref)"))
  (locals (HitVelocity :type "Float (double-precision)" :default 0.0) (IsValidHit :type Boolean) (KineticEnergy :type Integer64) (HitForceScale :type Integer64 :default 0))
  (if (not (`self.InCooldown`))
    (`|ExecutionSequence`
      (:`then_0`
        ;[1 1 1] Get the hit velocity and check if this exceeds a usable threshold.
        (set `local.HitForceScale` (`self.GetHitForceScale` (`local.SelfActor`) (`local.OtherActor`) (`local.NormalImpulse`)))
        (if (> (`local.HitForceScale`) 20)
          (set `local.IsValidHit` true)
          (set `self.InCooldown` true)
          (set `self.TimeSinceLastHit` 0.0)
          (else
            (return))))
      (:`then_1`
        ;[1 1 1] If the hit is valid, temporarily enable Tick for this component.
        (if (!= (`self.IsComponentTickEnabled`) (`local.IsValidHit`))
          (`self.SetComponentTickEnabled` (`local.IsValidHit`))))
      (:`then_2`))))

(fn `Initialize`
  (`|ExecutionSequence`
    (:`then_0`
      ;[1 1 1] get owner as StaticMeshActor.
      (bind _asstatic_mesh_actor (cast `StaticMeshActor` (`self.GetOwner`)))
      (set `self.StaticMesh` _asstatic_mesh_actor))
    (:`then_1`
      ;[1 1 1] get owner as StaticMeshActor.
      (add `Actor.OnActorHit` (`self.StaticMesh`) (`|CreateDelegate` :!event `HandleCollision`)))
    (:`then_2`
      ;[1 1 1] Add AudioComponent to owner.
      (bind _returnvalue (`|AddComponentByClass` :`self` (`self.GetOwner`) :`Class` "/Script/Engine.AudioComponent"))
      (bind _output_get (set `self.AudioComponent` _returnvalue))
      (`AudioComponent.SetSound` _output_get "/Game/CollisionSystem/MSS_CollisionAudioSource.MSS_CollisionAudioSource"))
    (:`then_3`
      (set `self.IsInitialized` true))))

(fn `SetMetaSoundAttributes`)

(fn `Update`
  (params (DeltaTime :type "Float (double-precision)"))
  (set `self.TimeSinceLastHit` (+ (`self.TimeSinceLastHit`) DeltaTime))
  (if (> (`self.TimeSinceLastHit`) (`self.CooldownInterval`))
    (set `self.InCooldown` false)
    (if (> (`self.TimeSinceLastHit`) 3.0)
      (`self.SetComponentTickEnabled` false)
      (`KismetSystemLibrary.PrintString` "Tick Disabled"))))