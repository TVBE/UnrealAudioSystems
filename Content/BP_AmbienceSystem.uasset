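; Procedural ambience Blueprint that plays randomized one-shot sounds from Preset data table rows, placed around a target.
; A single timer serves all rows: UpdateTimer plays the row with the lowest delay, rerolls it, then subtracts the new minimum from all delays.
; Each validated row supplies delay range, weighted or uniform sound choice, random offset with exclusion radius, and optional attenuation.
; GetSoundSource, meant to supply audio components, is empty here.
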(event `self.ReceiveBeginPlay`
  ;[1 1 1] Event BeginPlay
  (`self.Initialize`))

(fn `GetLocationAroundListener`
  (params (Target :type "Actor Object Reference") (Input :type "/Game/F_ProceduralSoundLocationData Structure") (UseActorOrientation :type Boolean))
  (returns (ReturnValue :type "Vector Structure"))
  (bind _returnvalue (`KismetMathLibrary.RandomFloatInRange` Input_ExclusionRadius_6_34A36D024295B37C6C5465A2F190FBE5 Input_HorizontalRange_2_16E1109C4AF533D2BBAE719904E35332))
  (bind _returnvalue_2 (`KismetMathLibrary.RandomFloatInRange` Input_ExclusionRadius_6_34A36D024295B37C6C5465A2F190FBE5 Input_HorizontalRange_2_16E1109C4AF533D2BBAE719904E35332))
  (bind _returnvalue_3 (`self.K2_GetActorLocation` Target))
  (bind _returnvalue_4 (`KismetMathLibrary.SelectFloat` (- 0.0 _returnvalue) _returnvalue (`KismetMathLibrary.RandomBool`)))
  (bind _returnvalue_5 (`KismetMathLibrary.SelectFloat` (- 0.0 _returnvalue_2) _returnvalue_2 (`KismetMathLibrary.RandomBool`)))
  (return (+ (`KismetMathLibrary.SelectVector` (+ _returnvalue_3 (+ (* (`self.GetActorRightVector` Target) _returnvalue_4) (* (`self.GetActorForwardVector` Target) _returnvalue_5))) (`KismetMathLibrary.MakeVector` (+ (.x _returnvalue_3) _returnvalue_5) (+ (.y _returnvalue_3) _returnvalue_4) (+ (.z _returnvalue_3) (`KismetMathLibrary.RandomFloatInRange` (* Input_VerticalRange_4_DF408AC5467EA3599BC71B94FC28F2EC -1.0) Input_VerticalRange_4_DF408AC5467EA3599BC71B94FC28F2EC))) UseActorOrientation) Input_Offset_9_D9A2BA1041AF766504C6B3811FF286E5)))

(fn `GetPresetAttributes`
  (params (Index :type Integer))
  (returns (ReturnData :type "/Game/F_ProceduralSoundData Structure") (IsValid :type Boolean))
  (locals (RowName :type Name) (NewLocalVar_0 :type "/Game/F_ProceduralSoundData Structure"))
  (bind ((`PrintToScreen_11_B20C0C724AA03D4831BC889327EB51C4` _printtoscreen) (`PrintToLog_10_550BCCED4A20E5B694FAEFB80CEC264B` _printtolog) (`TextColor_14_D5F8067B44E04854A75EBAAC4083FE83` _textcolor)) (break `/Game/F_ActorDebugSettings` (`self.DebugSettings`)))
  (bind ((`PrintToScreen_11_B20C0C724AA03D4831BC889327EB51C4` _printtoscreen_2) (`PrintToLog_10_550BCCED4A20E5B694FAEFB80CEC264B` _printtolog_2) (`TextColor_14_D5F8067B44E04854A75EBAAC4083FE83` _textcolor_2)) (break `/Game/F_ActorDebugSettings` (`self.DebugSettings`)))
  (bind _outrownames (`DataTableFunctionLibrary.GetDataTableRowNames` (`self.Preset`)))
  (set `local.RowName` (`|GetArrayItem` _outrownames (`local.Index`)))
  (bind _returnvalue (`|GetDataTableRow` (`self.Preset`) (`local.RowName`))
    (:`then`
      (if (`self.ValidateProceduralSoundData` _returnvalue)
        (return _returnvalue true)
        (else
          (if (>= (`KismetMathLibrary.Conv_ByteToInt` (`.DebugLevel_12_627A8404475EAF19BA152DAC6EF020B9` (break `/Game/F_ActorDebugSettings` (`self.DebugSettings`)))) 0)
            (`KismetSystemLibrary.PrintString` (`KismetTextLibrary.Conv_TextToString` (`|FormatText` (`KismetSystemLibrary.GetDisplayName` self) "{self}: DataTable {preset} row {index}: {rowname} contains invalid data! Ambience will not work for this row." (`KismetSystemLibrary.GetDisplayName` (`self.Preset`)) (`local.Index`) (`local.RowName`))) _printtoscreen_2 _printtolog_2 _textcolor_2 8.0))
          (return _returnvalue false))))
    (:`RowNotFound`
      (if (>= (`KismetMathLibrary.Conv_ByteToInt` (`.DebugLevel_12_627A8404475EAF19BA152DAC6EF020B9` (break `/Game/F_ActorDebugSettings` (`self.DebugSettings`)))) 0)
        (`KismetSystemLibrary.PrintString` (`KismetTextLibrary.Conv_TextToString` (`|FormatText` (`KismetSystemLibrary.GetDisplayName` self) "{self}: DataTable {preset} row {index}: {rowname} not found!" (`KismetSystemLibrary.GetDisplayName` (`self.Preset`)) (`local.Index`) (`local.RowName`))) _printtoscreen _printtolog _textcolor 8.0)))))

(fn `GetSoundSource`
  (returns (ReturnComponent :type "AudioComponent Object Reference"))
  (return null))

(fn `Initialize`
  (`|ExecutionSequence`
    (:`then_0`
      (`self.UpdateTimer`))
    (:`then_1`
      (set `self.IsInitialized` true))))

(fn `InitializeSoundSource`
  (params (InputData :type "/Game/F_ProceduralSoundData Structure"))
  (returns (ReturnSoundSource :type "AudioComponent Object Reference"))
  (locals (SoundSource :type "AudioComponent Object Reference"))
  (bind ((`Attenuation_16_9977ECF14C2D9853827283AA2CA9AD0C` _attenuation)) (break `/Game/F_ProceduralSoundData` (`local.InputData`)))
  (bind (_sounds _weigths) (break `/Game/F_ProceduralSoundData` (`local.InputData`)))
  (`|ExecutionSequence`
    (:`then_0`
      ;[1 1 1] Try to get available sound source. Create new audio component if none are available.
      (bind _returncomponent (`self.GetSoundSource`))
      (set `local.SoundSource` _returncomponent))
    (:`then_1`
      ;[1 1 1] Sets the location of the acquired AudioComponent.
      (`SceneComponent.K2_SetWorldLocation` (`local.SoundSource`) (`self.GetLocationAroundListener` null (`.PlayRange_22_6EB37C6E4DF62A309EB7DF807FEBEAB8` (break `/Game/F_ProceduralSoundData` (`local.InputData`)))) false false))
    (:`then_2`
      ;[1 1 1] Sets the sound of the acquired AudioComponent.
      (`AudioComponent.SetSound` (`local.SoundSource`) (select `bool` (`KismetArrayLibrary.Array_IsNotEmpty` _weigths) :`false` (`KismetArrayLibrary.Array_Random` _sounds) :`true` (`|GetArrayItem` _sounds (`self.RandomIntegerFromWeigths` _weigths)))))
    (:`then_3`
      ;[1 1 1] Overrides the attenuation if an attenuation asset is provided.
      (`/Engine/EditorBlueprintResources/StandardMacros.IsValid` _attenuation
        (:`Is Valid`
          (set `AudioComponent.AttenuationSettings` _attenuation (`local.SoundSource`)))))
    (:`then_4`
      (return (`local.SoundSource`)))))

(fn `RandomIntegerFromWeigths`
  (params (Input :type "Array of Integer"))
  (returns (ReturnValue :type Integer))
  (locals (RandVal :type Integer) (TotalChances :type Integer) (TotalChecked :type Integer) (ChosenInt :type Integer))
  (bind _output_get (set `local.TotalChances` (`self.TotalOfIntegerArray` Input)))
  (if (> _output_get 0)
    (set `local.RandVal` (`KismetMathLibrary.RandomIntegerInRange` 0 (- (`local.TotalChances`) 1)))
    (for (_array_element _array_index) (`local.Input`)
      (set `local.TotalChecked` (+ _array_element (`local.TotalChecked`)))
      (if (< (`local.RandVal`) (`local.TotalChecked`))
        (set `local.ChosenInt` _array_index)
        (break)))
    (else
      (set `local.ChosenInt` -1)))
  (return (`local.ChosenInt`)))

(fn `TotalOfIntegerArray`
  (params (Array :type "Array of Integer"))
  (returns (ReturnValue :type Integer))
  (locals (Total :type Integer))
  (bind _total (`local.Total`))
  (for _array_element Array
    (set `local.Total` (+ _total _array_element)))
  (return _total))

(fn `UpdateTimer`
  (locals (Index :type Integer) (PresetData :type "/Game/F_ProceduralSoundData Structure") (LowestValue :type "Float (single-precision)" :default 0.0))
  (bind (_sounds _weigths _attenuation _delaymax _delaymin) (break `/Game/F_ProceduralSoundData` (`local.PresetData`)))
  (`|ExecutionSequence`
    (:`then_0`
      ;[1 1 1] Get the lowest value inside delay array.
      (set `local.Index` (`KismetMathLibrary.MinOfFloatArray` (`self.Delays`))))
    (:`then_1`
      ;[1 1 1] Get attributes from data table.
      (bind (_returndata _isvalid) (`self.GetPresetAttributes` (`local.Index`)))
      (if _isvalid
        (set `local.PresetData` _returndata)
        (else
          (return))))
    (:`then_2`
      ;[1 1 1] Add new delay value to delay array.
      (`KismetArrayLibrary.Array_Set` (`self.Delays`) (`local.Index`) (`KismetMathLibrary.RandomFloatInRange` _delaymin _delaymax)))
    (:`then_3`
      ;[1 1 1] Initialize and play sound source
      (bind _returnsoundsource (`self.InitializeSoundSource` (`local.PresetData`)))
      (`AudioComponent.Play` _returnsoundsource 0.0))
    (:`then_4`
      ;[1 1 1] Update timer
      (bind _output_get (set `local.LowestValue` (`.MinValue` (`KismetMathLibrary.MinOfFloatArray` (`self.Delays`)))))
      (bind _returnvalue (`KismetSystemLibrary.K2_SetTimerDelegate` (`|CreateDelegate` :!event `UpdateTimer`) _output_get))
      (set `self.Timer` _returnvalue))
    (:`then_5`
      ;[1 1 1] Subtract lowest delay from all array values.
      (for (_array_element _array_index) (`self.Delays`)
        (`KismetArrayLibrary.Array_Set` (`self.Delays`) _array_index (- _array_element (`local.LowestValue`)))))))

(fn `UserConstructionScript`)

(fn `ValidateProceduralSoundData`
  (params (Input :type "/Game/F_ProceduralSoundData Structure"))
  (returns (ReturnValue :type Boolean))
  (bind (_sounds _weigths _attenuation _delaymax _delaymin _playrange) (break `/Game/F_ProceduralSoundData` Input))
  (bind (_offset _horizontalrange _verticalrange _exclusionradius) (break `/Game/F_ProceduralSoundLocationData` _playrange))
  ;[1 1 1] Checks certain struct values to ensure that data can be used.
  (return (and (`KismetArrayLibrary.Array_IsNotEmpty` _sounds) (> _delaymax 0.0) (> _delaymin 0.0) (>= _horizontalrange 0.0) (>= _verticalrange 0.0) (> _horizontalrange _exclusionradius))))