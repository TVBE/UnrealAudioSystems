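; Pooled sound source actor for the world ambience system that plays positioned sounds and releases itself back to its owning pool when playback finishes.
; Initialize stores the pool and binds the audio-finished callback; PlaySound moves the actor before playing.
; For object-aware sounds, it shuffles source classes and sphere-overlaps WorldStatic objects to play from a random match.
; Without a match, it uses the original transform or skips playback, as the data specifies.
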(event `PlaySound`
  (params (Sound :type "/Game/WorldAmbienceSystem/F_SoundSourceData Structure"))
  (bind (_transform _canplay) (`self.GetObjectAwareData` Sound))
  ;[1 1 1] Event Post Event
  (if (and (`KismetSystemLibrary.IsValid` (`.Sound_2_C278CD8D4793A03BEEDFF98E059309A8` (break `/Game/WorldAmbienceSystem/F_SoundSourceData` Sound))) _canplay)
    (`self.K2_SetActorLocation` self (.location _transform) false false)
    (`AudioComponent.Play` (`self.Audio`) 0.0)))

(event `Event OnAudioFinished`
  ;[1 1 1] Event Callback
  (set `self.IsPlaying` false)
  (`/Engine/EditorBlueprintResources/StandardMacros.IsValid` (`self.Pool`)
    (:`Is Valid`
      (`/Game/WorldAmbienceSystem/BPC_SoundSourceManager.ReleaseBackToPool` (`self.Pool`) self))))

(fn `GetObjectAwareData`
  (params (SoundSourceData :type "/Game/WorldAmbienceSystem/F_SoundSourceData Structure"))
  (returns (Transform :type "Transform Structure") (CanPlay :type Boolean))
  (bind (_sound _transform _isobjectaware _objectawarerange _sourceobjects _playifnoobjectisfound) (break `/Game/WorldAmbienceSystem/F_SoundSourceData` SoundSourceData))
  (if _isobjectaware
    (`KismetArrayLibrary.Array_Shuffle` _sourceobjects)
    (for _array_element _sourceobjects
      (bind (_outactors _returnvalue) (`KismetSystemLibrary.SphereOverlapActors` (.location _transform) (`KismetMathLibrary.Conv_IntToDouble` _objectawarerange) (`|MakeArray` "ObjectTypeQuery1" :!type "EObjectTypeQuery Enum") _array_element (`|MakeArray` self :!type "Actor Object Reference")))
      (if _returnvalue
        (return (`self.GetTransform` (`KismetArrayLibrary.Array_Random` _outactors)) true)))
    (if _playifnoobjectisfound
      (return (`.Transform_5_7E999D2B4E1BDF8B3A14F3B6A82B0B7C` (break `/Game/WorldAmbienceSystem/F_SoundSourceData` (`local.SoundSourceData`))) true)
      (else
        (return (struct) false)))
    (else
      (return _transform true))))

(fn `Initialize`
  (params (Pool :type "/Game/WorldAmbienceSystem/BPC_SoundSourceManager Object Reference"))
  (`|ExecutionSequence`
    (:`then_0`
      ;[1 1 1] Create a reference to the object pool that 'owns' this soundsource.
      (set `self.Pool` (`local.Pool`)))
    (:`then_1`
      ;[1 1 1] Subscribe to events.
      (add `AudioComponent.OnAudioFinished` (`self.Audio`) (`|CreateDelegate` :!event `Event OnAudioFinished`)))))

(fn `UserConstructionScript`)