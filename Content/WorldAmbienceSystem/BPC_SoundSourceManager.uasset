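; Component of BP_AmbienceSystem that manages pooled BP_SoundSource actors to play ambience sounds at given transforms.
; On BeginPlay, except on dedicated servers, it caches its owner and subscribes to its play-sound-source event.
; Play requests reuse the first pooled source or spawn and initialize a new one, with a release function returning sources to the pool.
; An optional debug sphere shows each play location.
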(event `self.ReceiveBeginPlay`
  ;[1 1 1] Event Begin Play
  (if (not (`KismetSystemLibrary.IsDedicatedServer`))
    (`self.Initialize`)))

(fn `Initialize`
  (`|ExecutionSequence`
    (:`then_0`
      ;[1 1 1] Get owner as BP_AmbienceSystem
      (bind _asbp_ambience_system (cast `/Game/WorldAmbienceSystem/BP_AmbienceSystem` (`self.GetOwner`)))
      (set `self.Owner` _asbp_ambience_system))
    (:`then_1`
      ;[1 1 1] Subscribe to events.
      (add `/Game/WorldAmbienceSystem/BP_AmbienceSystem.PlaySoundSource` (`self.Owner`) (`|CreateDelegate` :!event `Initialize Sound Source at Location`)))
    (:`then_2`
      (set `self.IsInitialized` true))))

(fn `Initialize Sound Source at Location`
  (params (SoundSourceData :type "/Game/WorldAmbienceSystem/F_SoundSourceData Structure") (Visualise :type Boolean) (Color :type "LinearColor Structure"))
  (`|ExecutionSequence`
    (:`then_0`
      (if (`KismetArrayLibrary.Array_IsValidIndex` (`self.Pool`))
        (`/Game/WorldAmbienceSystem/BP_SoundSource.PlaySound` (`|GetArrayItem` (`self.Pool`)) (`local.SoundSourceData`))
        (`KismetArrayLibrary.Array_Remove` (`self.Pool`))
        (else
          (bind _returnvalue (`|SpawnActorFromClass` "/Game/WorldAmbienceSystem/BP_SoundSource.BP_SoundSource_C" (`.Transform_5_7E999D2B4E1BDF8B3A14F3B6A82B0B7C` (break `/Game/WorldAmbienceSystem/F_SoundSourceData` (`local.SoundSourceData`))) "Undefined" "OverrideRootScale" null null))
          (`/Game/WorldAmbienceSystem/BP_SoundSource.Initialize` _returnvalue self)
          (`/Game/WorldAmbienceSystem/BP_SoundSource.PlaySound` _returnvalue (`local.SoundSourceData`)))))
    (:`then_1`
      (if (`local.Visualise`)
        (`KismetSystemLibrary.DrawDebugSphere` (.location (`.Transform_5_7E999D2B4E1BDF8B3A14F3B6A82B0B7C` (break `/Game/WorldAmbienceSystem/F_SoundSourceData` (`local.SoundSourceData`)))) 75.0 12 (`local.Color`) 4.0 6.0)))))

(fn `ReleaseBackToPool`
  (params (SoundSource :type "/Game/WorldAmbienceSystem/BP_SoundSource Object Reference (by ref)"))
  (`KismetArrayLibrary.Array_Add` (`self.Pool`) SoundSource))