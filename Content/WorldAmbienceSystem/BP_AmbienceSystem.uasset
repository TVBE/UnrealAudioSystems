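; Ambience system that plays procedural sounds around the player pawn from DataTable presets, initialized only off dedicated servers.
; Presets queue in a list, with the first active and the next taking over on removal.
; A single timer serves every row by waiting for the lowest random delay and subtracting it from the rest.
; Each firing picks a weighted sound, randomizes its location, checks height range and passes object-aware spawn data to playback.
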(event `self.ReceiveBeginPlay`
  ;[1 1 1] Event BeginPlay
  (if (not (`KismetSystemLibrary.IsDedicatedServer`))
    (`self.Initialize`)))

(fn `AddPresetToList`
  (params (Preset :type "DataTable Object Reference"))
  (`KismetArrayLibrary.Array_Add` (`self.PendingPresets`) Preset)
  (if (== (`KismetArrayLibrary.Array_Length` (`self.PendingPresets`)) 1)
    (`self.Set Preset` (`|GetArrayItem` (`self.PendingPresets`)))))

(fn `GetLocationAroundListener`
  (params (Target :type "Actor Object Reference") (Input :type "/Game/WorldAmbienceSystem/F_ProceduralSoundPlayRangeData Structure") (UseActorOrientation :type Boolean))
  (returns (ReturnValue :type "Vector Structure"))
  (bind _returnvalue (`KismetMathLibrary.RandomFloatInRange` Input_ExclusionRadius_6_34A36D024295B37C6C5465A2F190FBE5 Input_HorizontalRange_2_16E1109C4AF533D2BBAE719904E35332))
  (bind _returnvalue_2 (`KismetMathLibrary.RandomFloatInRange` Input_ExclusionRadius_6_34A36D024295B37C6C5465A2F190FBE5 Input_HorizontalRange_2_16E1109C4AF533D2BBAE719904E35332))
  (bind _returnvalue_3 (`self.K2_GetActorLocation` Target))
  (bind _returnvalue_4 (`KismetMathLibrary.SelectFloat` (- 0.0 _returnvalue) _returnvalue (`KismetMathLibrary.RandomBool`)))
  (bind _returnvalue_5 (`KismetMathLibrary.SelectFloat` (- 0.0 _returnvalue_2) _returnvalue_2 (`KismetMathLibrary.RandomBool`)))
  (return (+ (`KismetMathLibrary.SelectVector` (+ _returnvalue_3 (+ (* (`self.GetActorRightVector` Target) _returnvalue_4) (* (`self.GetActorForwardVector` Target) _returnvalue_5))) (`KismetMathLibrary.MakeVector` (+ (.x _returnvalue_3) _returnvalue_5) (+ (.y _returnvalue_3) _returnvalue_4) (+ (.z _returnvalue_3) (`KismetMathLibrary.RandomFloatInRange` (* Input_VerticalRange_4_DF408AC5467EA3599BC71B94FC28F2EC -1.0) Input_VerticalRange_4_DF408AC5467EA3599BC71B94FC28F2EC))) UseActorOrientation) Input_Offset_9_D9A2BA1041AF766504C6B3811FF286E5)))

(fn `GetPresetAttributes`
  (params (Index :type Integer))
  (returns (ReturnData :type "/Game/WorldAmbienceSystem/F_ProceduralSoundData Structure") (IsValid :type Boolean))
  (locals (RowName :type Name) (NewLocalVar_0 :type "/Game/WorldAmbienceSystem/F_ProceduralSoundData Structure"))
  (bind ((`PrintToScreen_11_B20C0C724AA03D4831BC889327EB51C4` _printtoscreen) (`PrintToLog_10_550BCCED4A20E5B694FAEFB80CEC264B` _printtolog) (`TextColor_14_D5F8067B44E04854A75EBAAC4083FE83` _textcolor)) (break `/Game/WorldAmbienceSystem/F_ActorDebugSettings` (`self.DebugSettings`)))
  (bind ((`PrintToScreen_11_B20C0C724AA03D4831BC889327EB51C4` _printtoscreen_2) (`PrintToLog_10_550BCCED4A20E5B694FAEFB80CEC264B` _printtolog_2) (`TextColor_14_D5F8067B44E04854A75EBAAC4083FE83` _textcolor_2)) (break `/Game/WorldAmbienceSystem/F_ActorDebugSettings` (`self.DebugSettings`)))
  (bind _outrownames (`DataTableFunctionLibrary.GetDataTableRowNames` (`self.Preset`)))
  (set `local.RowName` (`|GetArrayItem` _outrownames (`local.Index`)))
  (bind _returnvalue (`|GetDataTableRow` (`self.Preset`) (`local.RowName`))
    (:`then`
      (if (`self.ValidateProceduralSoundData` _returnvalue)
        (return _returnvalue true)
        (else
          (if (>= (`KismetMathLibrary.Conv_ByteToInt` (`.DebugLevel_12_627A8404475EAF19BA152DAC6EF020B9` (break `/Game/WorldAmbienceSystem/F_ActorDebugSettings` (`self.DebugSettings`)))) 1)
            (`KismetSystemLibrary.PrintString` (`KismetTextLibrary.Conv_TextToString` (`|FormatText` (`KismetSystemLibrary.GetDisplayName` self) "{self}: DataTable {preset} row {index}: {rowname} contains invalid data! Ambience will not work for this preset" (`KismetSystemLibrary.GetDisplayName` (`self.Preset`)) (`local.Index`) (`local.RowName`))) _printtoscreen_2 _printtolog_2 _textcolor_2 8.0))
          (return _returnvalue false))))
    (:`RowNotFound`
      (if (>= (`KismetMathLibrary.Conv_ByteToInt` (`.DebugLevel_12_627A8404475EAF19BA152DAC6EF020B9` (break `/Game/WorldAmbienceSystem/F_ActorDebugSettings` (`self.DebugSettings`)))) 0)
        (`KismetSystemLibrary.PrintString` (`KismetTextLibrary.Conv_TextToString` (`|FormatText` (`KismetSystemLibrary.GetDisplayName` self) "{self}: DataTable {preset} row {index}: {rowname} not found!" (`KismetSystemLibrary.GetDisplayName` (`self.Preset`)) (`local.Index`) (`local.RowName`))) _printtoscreen _printtolog _textcolor 8.0)))))

(fn `GetSoundSourceData`
  (params (InputData :type "/Game/WorldAmbienceSystem/F_ProceduralSoundData Structure"))
  (returns (Play :type Boolean) (SoundSourceData :type "/Game/WorldAmbienceSystem/F_SoundSourceData Structure"))
  (locals (LocalTransform :type "Transform Structure") (LocalSound :type "MetaSoundSource Object Reference") (CanPlay :type Boolean) (InRange :type Boolean))
  (bind (_sounds _delaymin _delaymax _playrange _modifiers _use) (break `/Game/WorldAmbienceSystem/F_ProceduralSoundData` (`local.InputData`)))
  (bind (_sounds_2 _delaymin_2 _delaymax_2 _playrange_2 _modifiers_2 _use_2) (break `/Game/WorldAmbienceSystem/F_ProceduralSoundData` (`local.InputData`)))
  (bind _returnvalue (`Controller.K2_GetPawn` (`GameplayStatics.GetPlayerController` 0)))
  (bind (_offset _horizontalrange _verticalrange _exclusionradius _heigthrange) (break `/Game/WorldAmbienceSystem/F_ProceduralSoundPlayRangeData` (`.PlayRange_22_6EB37C6E4DF62A309EB7DF807FEBEAB8` (break `/Game/WorldAmbienceSystem/F_ProceduralSoundData` (`local.InputData`)))))
  (bind (_sounds_3 _weights _objectawarespawning _objectawarerange _sourceobjects _playifnoobjectisfound) (break `/Game/WorldAmbienceSystem/F_SoundData` _sounds))
  (bind (_sounds_4 _weights_2) (break `/Game/WorldAmbienceSystem/F_SoundData` _sounds_2))
  (bind (_x _y) (`KismetMathLibrary.BreakVector2D` _heigthrange))
  (`|ExecutionSequence`
    (:`then_0`
      ;[1 1 1] Get sound transform.
      (`/Engine/EditorBlueprintResources/StandardMacros.IsValid` _returnvalue
        (:`Is Valid`
          (set `local.LocalTransform` (`KismetMathLibrary.MakeTransform` (`self.GetLocationAroundListener` _returnvalue (`.PlayRange_22_6EB37C6E4DF62A309EB7DF807FEBEAB8` (break `/Game/WorldAmbienceSystem/F_ProceduralSoundData` (`local.InputData`)))))))))
    (:`then_1`
      ;[1 1 1] Check wether this sound type is in range
      (set `local.InRange` (or (`KismetMathLibrary.InRange_FloatFloat` (.z (.location (`local.LocalTransform`))) _x _y) (== _heigthrange (0.0 0.0)))))
    (:`then_2`
      ;[1 1 1] Get sound event.
      (if _use_2
        (set `local.LocalSound` (`|GetArrayItem` _sounds_4 (`self.RandomIntegerFromWeigths` _weights_2)))))
    (:`then_3`
      (return (and (`local.InRange`) _use) (make `/Game/WorldAmbienceSystem/F_SoundSourceData` (`local.LocalSound`) (`local.LocalTransform`) _objectawarespawning _objectawarerange _sourceobjects _playifnoobjectisfound)))))

(fn `Initialize`
  (bind (_debugsettings_debuglevel _debugsettings_printtoscreen _debugsettings_printtolog _debugsettings_textcolor) (break `/Game/WorldAmbienceSystem/F_ActorDebugSettings` (`self.DebugSettings`)))
  (bind _debugsettings_debuglevel_2 (break `/Game/WorldAmbienceSystem/F_ActorDebugSettings` (`self.DebugSettings`)))
  (`|ExecutionSequence`
    (:`then_0`
      ;[1 1 1] Generate and store an arbitrary amount of random colors for debugging.
      (for _ (range 33)
        (`KismetArrayLibrary.Array_Add` (`self.DebugColors`) (make `LinearColor` (`KismetMathLibrary.RandomFloat`) (`KismetMathLibrary.RandomFloat`) (`KismetMathLibrary.RandomFloat`) 1.0))))
    (:`then_1`
      (set `self.IsInitialized` true)
      (if (>= (`KismetMathLibrary.Conv_ByteToInt` _debugsettings_debuglevel_2) 2)
        (`KismetSystemLibrary.PrintString` (`KismetTextLibrary.Conv_TextToString` (`|FormatText` self "{self}:AmbienceSystem initialization was succesful!")) _debugsettings_printtoscreen _debugsettings_printtolog _debugsettings_textcolor 8.0)))))

(fn `RandomIntegerFromWeigths`
  (params (Input :type "Array of Integer"))
  (returns (ReturnValue :type Integer))
  (locals (RandVal :type Integer) (TotalChances :type Integer) (TotalChecked :type Integer) (ChosenInt :type Integer))
  (bind _output_get (set `local.TotalChances` (`self.TotalOfIntegerArray` Input)))
  (if (> _output_get 0)
    (set `local.RandVal` (`KismetMathLibrary.RandomIntegerInRange` 0 (- (`local.TotalChances`) 1)))
    (for (_array_element _array_index) (`local.Input`)
      (set `local.TotalChecked` (+ _array_element (`local.TotalChecked`)))
      (if (< (`local.RandVal`) (`local.TotalChecked`))
        (set `local.ChosenInt` _array_index)
        (break)))
    (else
      (set `local.ChosenInt` -1)))
  (return (`local.ChosenInt`)))

(fn `RemovePresetFromList`
  (params (Preset :type "DataTable Object Reference"))
  (bind _debugsettings_debuglevel (break `/Game/WorldAmbienceSystem/F_ActorDebugSettings` (`self.DebugSettings`)))
  (bind ((`PrintToScreen_11_B20C0C724AA03D4831BC889327EB51C4` _printtoscreen) (`PrintToLog_10_550BCCED4A20E5B694FAEFB80CEC264B` _printtolog) (`TextColor_14_D5F8067B44E04854A75EBAAC4083FE83` _textcolor)) (break `/Game/WorldAmbienceSystem/F_ActorDebugSettings` (`self.DebugSettings`)))
  (`|ExecutionSequence`
    (:`then_0`
      (for (_array_element _array_index) (`self.PendingPresets`)
        (if (== _array_element Preset)
          (`|ExecutionSequence`
            (:`then_0`
              (break))
            (:`then_1`
              (`KismetArrayLibrary.Array_Remove` (`self.PendingPresets`) _array_index))))))
    (:`then_1`
      (if (and (== (`self.Preset`) Preset) (not (`KismetArrayLibrary.Array_Contains` (`self.PendingPresets`) Preset)))
        (if (`KismetArrayLibrary.Array_IsNotEmpty` (`self.PendingPresets`))
          (`self.Set Preset` (`|GetArrayItem` (`self.PendingPresets`)))
          (else
            (set `self.Preset` null)
            (if (`KismetSystemLibrary.K2_TimerExistsHandle` (`self.Timer`))
              (`KismetSystemLibrary.K2_ClearAndInvalidateTimerHandle` (`self.Timer`))
              (if (>= (`KismetMathLibrary.Conv_ByteToInt` _debugsettings_debuglevel) 2)
                (`KismetSystemLibrary.PrintString` (`KismetTextLibrary.Conv_TextToString` (`|FormatText` self "{self}: AmbienceSystem currently has no preset. Procedural ambience is paused")) _printtoscreen _printtolog _textcolor 8.0 "AmbiencePreset")))))))))

(fn `Set Preset`
  (params (Preset :type "DataTable Object Reference"))
  (bind _debugsettings_debuglevel (break `/Game/WorldAmbienceSystem/F_ActorDebugSettings` (`self.DebugSettings`)))
  (bind ((`PrintToScreen_11_B20C0C724AA03D4831BC889327EB51C4` _printtoscreen) (`PrintToLog_10_550BCCED4A20E5B694FAEFB80CEC264B` _printtolog) (`TextColor_14_D5F8067B44E04854A75EBAAC4083FE83` _textcolor)) (break `/Game/WorldAmbienceSystem/F_ActorDebugSettings` (`self.DebugSettings`)))
  (`|ExecutionSequence`
    (:`then_0`
      ;[1 1 1] Clear timer.
      (if (`KismetSystemLibrary.K2_TimerExistsHandle` (`self.Timer`))
        (`KismetSystemLibrary.K2_ClearAndInvalidateTimerHandle` (`self.Timer`))))
    (:`then_1`
      ;[1 1 1] Set preset DataTable.
      (set `self.Preset` (`local.Preset`)))
    (:`then_2`
      ;[1 1 1] Populate delay array with correct delay values.
      (`KismetArrayLibrary.Array_Clear` (`self.Delays`))
      (bind _outrownames (`DataTableFunctionLibrary.GetDataTableRowNames` (`self.Preset`)))
      (for (_ _array_index) _outrownames
        (bind (_returndata _isvalid) (`self.GetPresetAttributes` _array_index))
        (if _isvalid
          (bind ((`Sounds_39_5218E76044FC8E60DE38299AD8337C5F` _sounds) (`DelayMin_5_7A396866498984AB6BD0569A586200AE` _delaymin) (`DelayMax_3_7BA87F4D48A6C9D8D72C1CAD29DB149E` _delaymax)) (break `/Game/WorldAmbienceSystem/F_ProceduralSoundData` _returndata))
          (`KismetArrayLibrary.Array_Set` (`self.Delays`) _array_index (`KismetMathLibrary.RandomFloatInRange` _delaymin _delaymax) true)
          (else
            (return)))))
    (:`then_3`
      ;[1 1 1] Start timer.
      (`self.SetTimer`)
      (if (>= (`KismetMathLibrary.Conv_ByteToInt` _debugsettings_debuglevel) 2)
        (`KismetSystemLibrary.PrintString` (`KismetTextLibrary.Conv_TextToString` (`|FormatText` self "{self}: Ambience preset set to {preset}." (`self.Preset`))) _printtoscreen _printtolog _textcolor 8.0 "AmbiencePreset")))))

(fn `SetTimer`
  (locals (LowestValue :type "Float (single-precision)"))
  (`/Engine/EditorBlueprintResources/StandardMacros.IsValid` (`self.Preset`)
    (:`Is Valid`
      (`|ExecutionSequence`
        (:`then_0`
          ;[1 1 1] Update timer
          (bind _output_get (set `local.LowestValue` (`.MinValue` (`KismetMathLibrary.MinOfFloatArray` (`self.Delays`)))))
          (bind _returnvalue (`KismetSystemLibrary.K2_SetTimerDelegate` (`|CreateDelegate` :!event `Update`) _output_get))
          (set `self.Timer` _returnvalue))
        (:`then_1`
          ;[1 1 1] Subtract lowest delay from all array values.
          (for (_array_element _array_index) (`self.Delays`)
            (`KismetArrayLibrary.Array_Set` (`self.Delays`) _array_index (- _array_element (`local.LowestValue`)))))))))

(fn `TotalOfIntegerArray`
  (params (Array :type "Array of Integer"))
  (returns (ReturnValue :type Integer))
  (locals (Total :type Integer))
  (bind _total (`local.Total`))
  (for _array_element Array
    (set `local.Total` (+ _total _array_element)))
  (return _total))

(fn `Update`
  (locals (Index :type Integer) (PresetData :type "/Game/WorldAmbienceSystem/F_ProceduralSoundData Structure") (LowestValue :type "Float (single-precision)" :default 0.0))
  (bind _debugsettings_debuglevel (break `/Game/WorldAmbienceSystem/F_ActorDebugSettings` (`self.DebugSettings`)))
  (bind (_debugsettings_debuglevel_2 _debugsettings_printtoscreen _debugsettings_printtolog _debugsettings_textcolor) (break `/Game/WorldAmbienceSystem/F_ActorDebugSettings` (`self.DebugSettings`)))
  (bind _debugsettings_debuglevel_3 (break `/Game/WorldAmbienceSystem/F_ActorDebugSettings` (`self.DebugSettings`)))
  (bind (_sounds _delaymin _delaymax) (break `/Game/WorldAmbienceSystem/F_ProceduralSoundData` (`local.PresetData`)))
  (bind ((`PrintToScreen_11_B20C0C724AA03D4831BC889327EB51C4` _printtoscreen) (`PrintToLog_10_550BCCED4A20E5B694FAEFB80CEC264B` _printtolog) (`TextColor_14_D5F8067B44E04854A75EBAAC4083FE83` _textcolor)) (break `/Game/WorldAmbienceSystem/F_ActorDebugSettings` (`self.DebugSettings`)))
  (bind (_returndata _isvalid) (`self.GetPresetAttributes` (`local.Index`)))
  (bind (_play _soundsourcedata) (`self.GetSoundSourceData` (`local.PresetData`)))
  (`|ExecutionSequence`
    (:`then_0`
      ;[1 1 1] Get the lowest value inside delay array.
      (set `local.Index` (`KismetMathLibrary.MinOfFloatArray` (`self.Delays`))))
    (:`then_1`
      ;[1 1 1] Get attributes from data table.
      (if _isvalid
        (set `local.PresetData` _returndata)
        (else
          (return))))
    (:`then_2`
      ;[1 1 1] Add new delay value to delay array.
      (`KismetArrayLibrary.Array_Set` (`self.Delays`) (`local.Index`) (`KismetMathLibrary.RandomFloatInRange` _delaymin _delaymax)))
    (:`then_3`
      ;[1 1 1] Call  PlaySound.
      (`/Engine/EditorBlueprintResources/StandardMacros.IsValid` (`Controller.K2_GetPawn` (`GameplayStatics.GetPlayerController` 0))
        (:`Is Valid`
          (if _play
            (`self.PlaySoundSource` _soundsourcedata (>= (`KismetMathLibrary.Conv_ByteToInt` _debugsettings_debuglevel_3) 2) (`|GetArrayItem` (`self.DebugColors`) (`local.Index`)))
            (elif (and (>= (`KismetMathLibrary.Conv_ByteToInt` _debugsettings_debuglevel) 2) (not (`.Use_30_AA44C4934E269130DD6BABB1A4EB3764` (break `/Game/WorldAmbienceSystem/F_ProceduralSoundData` (`local.PresetData`)))))
              (bind _outrownames (`DataTableFunctionLibrary.GetDataTableRowNames` (`self.Preset`)))
              (`KismetSystemLibrary.PrintString` (`KismetTextLibrary.Conv_TextToString` (`|FormatText` self "{self}: {row}  was skipped since flag 'use' was set to false." (`|GetArrayItem` _outrownames (`local.Index`)))) _debugsettings_printtoscreen _debugsettings_printtolog _debugsettings_textcolor 8.0 "None"))))
        (:`Is Not Valid`
          (if (>= (`KismetMathLibrary.Conv_ByteToInt` (`.DebugLevel_12_627A8404475EAF19BA152DAC6EF020B9` (break `/Game/WorldAmbienceSystem/F_ActorDebugSettings` (`self.DebugSettings`)))) 0)
            (`KismetSystemLibrary.PrintString` (`KismetTextLibrary.Conv_TextToString` (`|FormatText` (`KismetSystemLibrary.GetDisplayName` self) "{self}: No player pawn found! Ambience will not spawn.")) _printtoscreen _printtolog _textcolor 8.0)))))
    (:`then_4`
      ;[1 1 1] Update the timer.
      (`self.SetTimer`))))

(fn `UserConstructionScript`)

(fn `ValidateProceduralSoundData`
  (params (Input :type "/Game/WorldAmbienceSystem/F_ProceduralSoundData Structure"))
  (returns (ReturnValue :type Boolean))
  (bind (_sounds _delaymin _delaymax _playrange) (break `/Game/WorldAmbienceSystem/F_ProceduralSoundData` Input))
  (bind (_offset _horizontalrange _verticalrange _exclusionradius) (break `/Game/WorldAmbienceSystem/F_ProceduralSoundPlayRangeData` _playrange))
  ;[1 1 1] Checks certain struct values to ensure that data can be used.
  (return (and (`KismetArrayLibrary.Array_IsNotEmpty` (`.Sounds_3_F305A1214E460D65017DC4A6B1A69FEC` (break `/Game/WorldAmbienceSystem/F_SoundData` _sounds))) (> _delaymax 0.0) (> _delaymin 0.0) (>= _horizontalrange 0.0) (>= _verticalrange 0.0) (> _horizontalrange _exclusionradius))))